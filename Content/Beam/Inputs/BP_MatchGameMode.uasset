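; BP_MatchGameMode is the game mode for a match, linking match start and end to the Beam game instance.
; On BeginPlay it caches BP_BeamGameInstance and calls its reload event, then waits a tick and sets the first player's view target to the BP_GlobalCamera actor.
; When the match ends, it forwards the event to the game instance's match-end handler.
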(event `self.ReceiveBeginPlay`
  (bind _asbp_beam_game_instance (cast `/Game/Beam/BP_BeamGameInstance` (`GameplayStatics.GetGameInstance`))
    (:`then`
      (bind _output_get (set `self.As BP Beam Game Instance` _asbp_beam_game_instance))
      (`/Game/Beam/BP_BeamGameInstance.CE_Reload` _output_get))
    (:`CastFailed`
      _))
  (`KismetSystemLibrary.DelayUntilNextTick`)
  (bind _returnvalue (`GameplayStatics.GetActorOfClass` "/Game/Beam/Blueprints/BP_GlobalCamera.BP_GlobalCamera_C"))
  (`PlayerController.SetViewTargetWithBlend` (`GameplayStatics.GetPlayerController` 0) _returnvalue 0.0 "VTBlend_Linear" 0.0 false))

(event `self.WhenMatchEnd`
  (`/Game/Beam/BP_BeamGameInstance.CE_OnMatchEnd` (`self.As BP Beam Game Instance`)))

(fn `UserConstructionScript`)