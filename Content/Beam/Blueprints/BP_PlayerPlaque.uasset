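; BP_PlayerPlaque is a pad that registers the BP_BeamCharacter standing on it, resetting that character's life and setting up its skin.
; When the registered player leaves, it clears the reference and hides its visuals.
; It exposes functions to show a Niagara barrier with X/Y/Z counts and to drive a remapped percentage on Cube1's dynamic "Digital" material.
; HideNiagara, also run at BeginPlay, clears both effects.
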(event `self.ReceiveBeginPlay`
  (bind _returnvalue (`PrimitiveComponent.CreateDynamicMaterialInstance` (`self.Cube1`) 0 "/Game/Beam/Asset/VFX/Transform/Digital.Digital" "None"))
  (set `self.digital` _returnvalue)
  (`self.HideNiagara`))

(event `self.ReceiveActorBeginOverlap`
  (params (OtherActor :type "Actor Object Reference"))
  (bind _asbp_beam_character (cast `/Game/Beam/Blueprints/BP_BeamCharacter` OtherActor))
  (bind _output_get (set `self.player` _asbp_beam_character))
  (`KismetSystemLibrary.PrintString` "ENTERED PLAQUE")
  (`BeamCharacter.ResetLife` _output_get)
  (`/Game/Beam/Blueprints/BP_BeamCharacter.SetupSkin` _output_get))

(event `self.ReceiveActorEndOverlap`
  (params (OtherActor :type "Actor Object Reference"))
  (bind _asbp_beam_character (cast `/Game/Beam/Blueprints/BP_BeamCharacter` OtherActor))
  (if (== _asbp_beam_character (`self.player`))
    (set `self.player` null)
    (`KismetSystemLibrary.PrintString` "LEFT PLAQUE")
    (`self.HideNiagara`)))

(fn `HideNiagara`
  (`NiagaraComponent.SetAsset` (`self.Barrier`) null true)
  (`MaterialInstanceDynamic.SetScalarParameterValue` (`self.digital`) "Pourcentage" -0.2))

(fn `RenderDigital`
  (params (percent :type "Float (double-precision) (by ref)"))
  (`MaterialInstanceDynamic.SetScalarParameterValue` (`self.digital`) "Pourcentage" (/ (- percent 0.3) 1.7)))

(fn `RenderNiagara`
  (params (X :type "Integer (by ref)") (Y :type "Integer (by ref)") (Z :type "Integer (by ref)"))
  (bind _barrier (`self.Barrier`))
  (`NiagaraComponent.SetAsset` _barrier (`self.niagaraAsset`) true)
  (`NiagaraComponent.SetVariableInt` _barrier "XCount" X)
  (`NiagaraComponent.SetVariableInt` _barrier "YCount" Y)
  (`NiagaraComponent.SetVariableInt` _barrier "ZCount" Z))

(fn `UserConstructionScript`)