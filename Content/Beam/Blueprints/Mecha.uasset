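; Mecha actor that shoves nearby BeamCharacters and knocks itself back when it touches obstacles along the X axis.
; Two box overlaps track a single BeamCharacter, and pressing E knocks it away from the Mecha in the XZ plane.
; Every tick, short line traces on both X sides trigger a self-knockback in a fixed +X/+Z direction.
; A state-machine check for Fall is left unconnected.
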(event `self.ReceiveTick`
  (params (DeltaSeconds :type "Float (single-precision)"))
  (bind _returnvalue (`self.K2_GetActorLocation`))
  (bind (_outhit _returnvalue_2) (`KismetSystemLibrary.LineTraceSingle` _returnvalue (+ _returnvalue (20.0 0.0 0.0)) "TraceTypeQuery1"))
  (bind (_outhit_2 _returnvalue_3) (`KismetSystemLibrary.LineTraceSingle` _returnvalue (- _returnvalue (20.0 0.0 0.0)) "TraceTypeQuery1"))
  (if (or _returnvalue_2 _returnvalue_3)
    (`self.KnockBack` (1.0 0.0 1.0) 10.0)))

(event `Key|E`
  (params (Key :type "Key Structure"))
  (bind _actorin (`self.ActorIn`))
  (:`Pressed`
    (if (`KismetSystemLibrary.IsValid` _actorin)
      (bind _asbeam_character (cast `BeamCharacter` _actorin))
      (`self.KnockBack` _asbeam_character (`KismetMathLibrary.MakeVector` (.x (- (`self.K2_GetActorLocation` _actorin) (`self.K2_GetActorLocation`))) 0.0 (.z (- (`self.K2_GetActorLocation` _actorin) (`self.K2_GetActorLocation`)))) 10.0))))

(event `self.Box1.OnComponentBeginOverlap`
  (params (OverlappedComponent :type "PrimitiveComponent Object Reference") (OtherActor :type "Actor Object Reference") (OtherComp :type "PrimitiveComponent Object Reference") (OtherBodyIndex :type Integer) (bFromSweep :type Boolean) (SweepResult :type "HitResult Structure (by ref)"))
  (`self.Enter` OtherActor))

(event `self.Box1.OnComponentEndOverlap`
  (params (OverlappedComponent :type "PrimitiveComponent Object Reference") (OtherActor :type "Actor Object Reference") (OtherComp :type "PrimitiveComponent Object Reference") (OtherBodyIndex :type Integer))
  (`self.End` OtherActor))

(event `self.Box.OnComponentBeginOverlap`
  (params (OverlappedComponent :type "PrimitiveComponent Object Reference") (OtherActor :type "Actor Object Reference") (OtherComp :type "PrimitiveComponent Object Reference") (OtherBodyIndex :type Integer) (bFromSweep :type Boolean) (SweepResult :type "HitResult Structure (by ref)"))
  (`self.Enter` OtherActor))

(event `self.Box.OnComponentEndOverlap`
  (params (OverlappedComponent :type "PrimitiveComponent Object Reference") (OtherActor :type "Actor Object Reference") (OtherComp :type "PrimitiveComponent Object Reference") (OtherBodyIndex :type Integer))
  (`self.End` OtherActor))

(fn `UserConstructionScript`)