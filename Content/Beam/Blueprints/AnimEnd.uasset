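; Beam actor that plays an end animation on a given character, with a cinematic camera and a laser sound.
; AnimEnd locks camera state, follows the character and parks the actor diagonally above them.
; After a timer, Tick frees the camera, jitters it randomly around the character, stretches the beam and aims the cube along the actor-to-character direction.
; StopAnim unlocks and reverses the cinematic, but leaves the timer and start flag set.
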(event `self.ReceiveBeginPlay`
  (bind _returnvalue (`GameplayStatics.GetActorOfClass` "/Game/Beam/Blueprints/BP_GlobalCamera.BP_GlobalCamera_C"))
  (set `self.camera` _returnvalue))

(event `self.ReceiveTick`
  (params (DeltaSeconds :type "Float (single-precision)"))
  (bind _returnvalue (subsystem `CameraWorldSubsystem`))
  (bind _beameffect (`self.BeamEffect`))
  (bind _x (.x (`self.K2_GetActorLocation` (`self.Character`))))
  (bind _z (.z (`self.K2_GetActorLocation` (`self.Character`))))
  (if (`self.End`)
    (if (`self.StartAnim`)
      (`SceneComponent.SetWorldScale3D` _beameffect (`KismetMathLibrary.MakeVector` (.x (`SceneComponent.K2_GetComponentScale` _beameffect)) (.y (`SceneComponent.K2_GetComponentScale` _beameffect)) (`KismetMathLibrary.FInterpTo` (.z (`SceneComponent.K2_GetComponentScale` _beameffect)) 100.0 DeltaSeconds 0.1)))
      (`CameraWorldSubsystem.ChangeCameraMode` _returnvalue "Free")
      (`self.K2_SetActorLocation` (`self.camera`) (`KismetMathLibrary.MakeVector` (`KismetMathLibrary.FInterpTo` _x (+ _x (`KismetMathLibrary.RandomFloatInRange` -200.0 200.0)) DeltaSeconds 50.0) (`self.Y`) (`KismetMathLibrary.FInterpTo` _z (+ _z (`KismetMathLibrary.RandomFloatInRange` -200.0 200.0)) DeltaSeconds 50.0)) false false)
      (`SceneComponent.K2_SetWorldRotation` (`self.Cube`) (`KismetMathLibrary.MakeRotFromX` (- (`self.K2_GetActorLocation` (`self.Character`)) (`self.K2_GetActorLocation`))) false false)
      (`self.K2_SetActorLocation` (`KismetMathLibrary.MakeVector` (+ (.x (`self.K2_GetActorLocation` (`self.Character`))) 2000.0) (.y (`self.K2_GetActorLocation` (`self.Character`))) (+ (.z (`self.K2_GetActorLocation` (`self.Character`))) 2000.0)))
      (else
        (bind _output_get (set `self.timer` (+ (`self.timer`) DeltaSeconds)))
        (if (> _output_get (`self.timeMax`))
          (`CameraWorldSubsystem.ChangeCameraMode` _returnvalue "Free")
          (set `self.StartAnim` true)
          (set `self.Y` (.y (`self.K2_GetActorLocation` (`self.camera`)))))))))

(fn `AnimEnd`
  (params (Character :type "/Game/Beam/Blueprints/BP_BeamCharacter Object Reference"))
  (bind _returnvalue (subsystem `CameraWorldSubsystem`))
  (set `self.Character` Character)
  (`CameraWorldSubsystem.CameraCinematic` _returnvalue 2.0 (0.0 0.0 0.0) Character false 350.0)
  (`CameraWorldSubsystem.SetCanChangeState` _returnvalue false)
  (`self.K2_SetActorLocation` (`KismetMathLibrary.MakeVector` (+ (.x (`self.K2_GetActorLocation` Character)) 2000.0) (.y (`self.K2_GetActorLocation` Character)) (+ (.z (`self.K2_GetActorLocation` Character)) 2000.0)))
  (set `self.End` true)
  ;[1 1 1] Mettre un son de loop de mega laser
  (`AkGameplayStatics.PostEvent` "/Game/WwiseAudio/Events/Default_Work_Unit/SFX/Gun/Play_SFX_Gun_Shoot3.Play_SFX_Gun_Shoot3"))

(fn `StopAnim`
  (`KismetSystemLibrary.PrintString` "STIO ANIM END")
  (`CameraWorldSubsystem.SetCanChangeState` (subsystem `CameraWorldSubsystem`) true)
  (`CameraWorldSubsystem.ReverseCinematic` (subsystem `CameraWorldSubsystem`) 5.0)
  (set `self.End` false))

(fn `UserConstructionScript`)