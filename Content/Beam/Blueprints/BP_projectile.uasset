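; BP_projectile is a projectile actor in the Beam folder, sized and propelled by a parameter struct.
; Its InitParameters event applies the current speed to the projectile component as max speed and local forward velocity.
; The same event scales the cylinder mesh by width and height and resizes the capsule to match.
; Emitter spawn and OwnPower switch nodes are present but never run.
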(event `self.InitParameters`
  (bind (_projectilecurrentparam_speed _projectilecurrentparam_width _projectilecurrentparam_height) (break `ProjectileParameters` (`self.projectileCurrentParam`)))
  (bind _capsule (`self.Capsule`))
  (bind _projectilecomponent (`self.projectileComponent`))
  (set `ProjectileMovementComponent.MaxSpeed` _projectilecurrentparam_speed _projectilecomponent)
  (`ProjectileMovementComponent.SetVelocityInLocalSpace` _projectilecomponent (`KismetMathLibrary.MakeVector` _projectilecurrentparam_speed))
  (`SceneComponent.SetRelativeScale3D` (`self.Cylinder`) (`KismetMathLibrary.MakeVector` _projectilecurrentparam_width _projectilecurrentparam_width _projectilecurrentparam_height))
  (`CapsuleComponent.SetCapsuleRadius` _capsule (* _projectilecurrentparam_width 50.0) true)
  (`CapsuleComponent.SetCapsuleHalfHeight` _capsule (* _projectilecurrentparam_height 50.0) true))

(fn `UserConstructionScript`)