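; StartScene opens a match, running the intro beat and managing music and ambience through Wwise.
; BeginPlay starts step-one music and crowd ambience, then a tick later updates beam character outlines and freezes players under camera shake for a few seconds before releasing them.
; Music change events advance a three-step track sequence by stopping the current track and starting the next, while a music end event stops all steps.
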(event `self.ReceiveBeginPlay`
  (bind _returnvalue (subsystem `CameraWorldSubsystem`))
  (`AkGameplayStatics.PostEvent` "/Game/WwiseAudio/Events/Default_Work_Unit/MUSIC/Step1/Play_Music_step_1.Play_Music_step_1" self)
  (`AkGameplayStatics.SetRTPCValue` "/Game/WwiseAudio/Game_Parameters/Default_Work_Unit/Volume_Music.Volume_Music" 25.0)
  (`AkGameplayStatics.PostEvent` "/Game/WwiseAudio/Events/Default_Work_Unit/AMB/Play_AMB_Arena_Crowd_Loop.Play_AMB_Arena_Crowd_Loop" self)
  (set `self.MusicStep` 1)
  (`KismetSystemLibrary.DelayUntilNextTick`)
  (bind _asmatch_game_mode (cast `MatchGameMode` (`GameplayStatics.GetGameMode`)))
  (bind _output_get (set `self.AsMatchGameMode` _asmatch_game_mode))
  (bind _outactors (`GameplayStatics.GetAllActorsOfClass` "/Game/Beam/Blueprints/BP_BeamCharacter.BP_BeamCharacter_C"))
  (for _array_element _outactors
    (bind _asbp_beam_character (cast `/Game/Beam/Blueprints/BP_BeamCharacter` _array_element))
    (`/Game/Beam/Blueprints/BP_BeamCharacter.ChangeOutlineColor` _asbp_beam_character))
  (`MatchGameMode.FreezePlayers` _output_get)
  (`CameraWorldSubsystem.ShakeCamera` _returnvalue 30.0 20.0)
  (`KismetSystemLibrary.Delay` 4.0)
  (`MatchGameMode.UnFreezePlayers` _output_get)
  (`CameraWorldSubsystem.UnShakeCamera` _returnvalue))

(event `OnMusicChange`
  (switch `int` (`self.MusicStep`)
    (:`1`
      (set `self.MusicStep` 2)
      (`AkGameplayStatics.PostEvent` "/Game/WwiseAudio/Events/Default_Work_Unit/MUSIC/Step1/Stop_Music_step_1.Stop_Music_step_1" self)
      (`AkGameplayStatics.PostEvent` "/Game/WwiseAudio/Events/Default_Work_Unit/MUSIC/Step2/Play_Music_step_2.Play_Music_step_2" self))
    (:`2`
      (set `self.MusicStep` 3)
      (`AkGameplayStatics.PostEvent` "/Game/WwiseAudio/Events/Default_Work_Unit/MUSIC/Step2/Stop_Music_step_2.Stop_Music_step_2" self)
      (`AkGameplayStatics.PostEvent` "/Game/WwiseAudio/Events/Default_Work_Unit/MUSIC/Step3/Play_Music_step_3.Play_Music_step_3" self))))

(event `OnMusicEnd`
  (`AkGameplayStatics.PostEvent` "/Game/WwiseAudio/Events/Default_Work_Unit/MUSIC/Step1/Stop_Music_step_1.Stop_Music_step_1" self)
  (`AkGameplayStatics.PostEvent` "/Game/WwiseAudio/Events/Default_Work_Unit/MUSIC/Step2/Stop_Music_step_2.Stop_Music_step_2" self)
  (`AkGameplayStatics.PostEvent` "/Game/WwiseAudio/Events/Default_Work_Unit/MUSIC/Step3/Stop_Music_step_3.Stop_Music_step_3" self))

(fn `UserConstructionScript`)