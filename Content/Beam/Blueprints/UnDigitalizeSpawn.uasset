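; UnDigitalizeSpawn is a short-lived effect actor that animates a digital material on a sphere, then destroys itself.
; BeginPlay creates a dynamic instance of the Digital material, sets its Pourcentage parameter to full and prints a debug message.
; Tick counts Timer down slightly faster than real time, scales it by MaxSecs and MaxValue into Pourcentage, and destroys the actor once Timer falls to minus one.
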(event `self.ReceiveBeginPlay`
  (`KismetSystemLibrary.PrintString` "Hello")
  (bind _returnvalue (`PrimitiveComponent.CreateDynamicMaterialInstance` (`self.Sphere`) 0 "/Game/Beam/Asset/VFX/Transform/Digital.Digital" "None"))
  (bind _output_get (set `self.material` _returnvalue))
  (`MaterialInstanceDynamic.SetScalarParameterValue` _output_get "Pourcentage" 1.0))

(event `self.ReceiveTick`
  (params (DeltaSeconds :type "Float (single-precision)"))
  (bind _output_get (set `self.Timer` (- (`self.Timer`) (* DeltaSeconds 1.2))))
  (`MaterialInstanceDynamic.SetScalarParameterValue` (`self.material`) "Pourcentage" (- (* (/ _output_get (`self.maxSecs`)) (`self.maxValue`)) 0.0))
  (if (>= -1.0 (`self.Timer`))
    (`self.K2_DestroyActor`)))

(fn `Hello`)

(fn `UserConstructionScript`)