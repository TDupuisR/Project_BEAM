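; Trigger actor that swaps the skins of beam characters standing together inside it.
; Overlap events add and remove BP_BeamCharacter actors from a Players list.
; While at least two are inside, Tick runs a timer that resets otherwise; on reaching TimeMax it toggles each character's SkinIndex between 0 and 1 and calls SetupSkin.
; Debug strings print on entry, exit and each swap.
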(event `self.ReceiveTick`
  (params (DeltaSeconds :type "Float (single-precision)"))
  (if (>= (`KismetArrayLibrary.Array_Length` (`self.players`)) 2)
    (bind _output_get (set `self.timer` (+ (`self.timer`) DeltaSeconds)))
    (if (>= _output_get (`self.timeMax`))
      (set `self.timer` 0.0)
      (for _array_element (`self.players`)
        ;[0 0 0] Faut att le truc (si 1 -> 0, si 0 -> 1)
        (`self.ChangeSkin` _array_element)
        (`/Game/Beam/Blueprints/BP_BeamCharacter.SetupSkin` _array_element)
        (`KismetSystemLibrary.PrintString` "CHANGE SKIN" true true (struct :`R` 1.0 :`B` 0.254646 :`A` 1.0) 5.0)))
    (else
      (set `self.timer` 0.0))))

(event `self.ReceiveActorBeginOverlap`
  (params (OtherActor :type "Actor Object Reference"))
  (bind _asbp_beam_character (cast `/Game/Beam/Blueprints/BP_BeamCharacter` OtherActor))
  (`KismetArrayLibrary.Array_Add` (`self.players`) _asbp_beam_character)
  (`KismetSystemLibrary.PrintString` "ADDED"))

(event `self.ReceiveActorEndOverlap`
  (params (OtherActor :type "Actor Object Reference"))
  (bind _asbp_beam_character (cast `/Game/Beam/Blueprints/BP_BeamCharacter` OtherActor))
  (`KismetArrayLibrary.Array_RemoveItem` (`self.players`) _asbp_beam_character)
  (`KismetSystemLibrary.PrintString` "REMOVED"))

(fn `UserConstructionScript`)