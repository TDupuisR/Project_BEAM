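; Beam game instance that owns the shared UI widgets and handles level loading and round transitions.
; Init creates loading, end-round, debug, pause and option widgets; CE_Reload re-adds the transition widgets and finishes the stored transition type, normal load or match round.
; Round end freezes players, animates a dead character, then renders the end-round widget.
; GetNewRoundMap shuffles the level list and avoids repeating the current map.
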(event `CE_Reload`
  (if (not (`self.DisableUI`))
    (`KismetSystemLibrary.DelayUntilNextTick`)
    (`KismetSystemLibrary.Delay` 0.01)
    (`UserWidget.AddToViewport` (`self.Widget End Round`) 0)
    (`UserWidget.AddToViewport` (`self.LoadingScreen`) 0)
    (if (`self.DebugUI`)
      (`UserWidget.AddToViewport` (`self.WidgetDebug`) 0))
    (`KismetSystemLibrary.DelayUntilNextTick`)
    (switch `/Game/Beam/Blueprints/Enum_SceneTransition` (`self.TransitionType`)
      (:`NewEnumerator2`
        _)
      (:`NewEnumerator1`
        (`self.CE_OnEndLoadScreen`))
      (:`NewEnumerator0`
        (`self.CE_OnRoundRestart`)))
    (set `self.TransitionType` "NewEnumerator2")))

(event `self.ReceiveInit`
  (bind _returnvalue (`GameplayStatics.GetPlayerController` 0))
  (if (`self.DebugUI`)
    (`KismetSystemLibrary.ExecuteConsoleCommand` "ENABLEALLSCREENMESSAGES" null)
    (else
      (`KismetSystemLibrary.ExecuteConsoleCommand` "DISABLEALLSCREENMESSAGES" null)))
  (`KismetSystemLibrary.DelayUntilNextTick`)
  (if (not (`self.DisableUI`))
    (bind _ascore_hud (cast `/Game/Eng/UI/Core_HUD` (`PlayerController.GetHUD` (`GameplayStatics.GetPlayerController` 0))))
    (set `self.Core HUD` _ascore_hud)
    (bind _returnvalue_2 (`|CreateWidget` "/Game/Eng/UI/W_LoadingScreen.W_LoadingScreen_C" (`GameplayStatics.GetPlayerController` 0)))
    (bind _output_get (set `self.LoadingScreen` _returnvalue_2))
    (`UserWidget.AddToViewport` _output_get -5)
    (bind _returnvalue_3 (`|CreateWidget` "/Game/WidgetEndRound.WidgetEndRound_C" (`GameplayStatics.GetPlayerController` 0)))
    (bind _output_get_2 (set `self.Widget End Round` _returnvalue_3))
    (`Widget.SetVisibility` _output_get_2 "HitTestInvisible")
    (bind _returnvalue_4 (`|CreateWidget` "/Game/WidgetDebut.WidgetDebut_C" (`GameplayStatics.GetPlayerController` 0)))
    (set `self.WidgetDebug` _returnvalue_4)
    (bind _returnvalue_5 (`|CreateWidget` "/Game/Eng/UI/W_PauseMenu.W_PauseMenu_C" _returnvalue))
    (set `self.Pause Menu` _returnvalue_5)
    (bind _returnvalue_6 (`|CreateWidget` "/Game/Eng/UI/W_Option.W_Option_C" _returnvalue))
    (set `self.Option Menu` _returnvalue_6)))

(event `CE_OnRoundEnd`
  (`self.FreezeEnd`)
  (`self.AnimFinale`)
  (`KismetSystemLibrary.Delay` 3.5)
  (if (not (`self.DisableUI`))
    (`/Game/WidgetEndRound.Render` (`self.Widget End Round`))))

(event `CE_OnRoundRestart`
  (if (not (`self.DisableUI`))
    (`/Game/WidgetEndRound.CE_OpeningAnimation` (`self.Widget End Round`))
    (bind _returnvalue (`GameplayStatics.GetActorOfClass` "/Game/Beam/Blueprints/AnimEnd.AnimEnd_C"))
    (`/Game/Beam/Blueprints/AnimEnd.StopAnim` _returnvalue)))

(event `CE_OnLoadScreen`
  (if (not (`self.DisableUI`))
    (`/Game/Eng/UI/W_LoadingScreen.CE_Appear` (`self.LoadingScreen`))))

(event `CE_OnEndLoadScreen`
  (if (not (`self.DisableUI`))
    (`/Game/Eng/UI/W_LoadingScreen.CE_Disappear` (`self.LoadingScreen`))
    (`/Game/WidgetEndRound.CE_ResetVisuals` (`self.Widget End Round`) true)
    (`MatchSystemBeam.ResetPlayerPoints` (`self.GetMancheSystem`))))

(event `CE_LoadingScene`
  (params (Transition :type "/Game/Beam/Blueprints/Enum_SceneTransition Enum" :default "NewEnumerator1") (Level :type "World Soft Object Reference"))
  (bind _output_get (set `self.TransitionType` Transition))
  (switch `/Game/Beam/Blueprints/Enum_SceneTransition` _output_get
    (:`NewEnumerator2`
      _)
    (:`NewEnumerator1`
      (if (not (`self.DisableUI`))
        (`self.CE_OnLoadScreen`)
        (`KismetSystemLibrary.Delay` 1.0))
      (if (== Level (`self.Compare`))
        (`MatchSystemBeam.ResetPlayerPoints` (`self.GetMancheSystem`))))
    (:`NewEnumerator0`
      _))
  (`GameplayStatics.OpenLevelBySoftObjectPtr` Level false))

(event `CE_Add Widget Pause`
  (if (not (`self.DisableUI`))
    (`UserWidget.AddToViewport` (`self.Pause Menu`) 0)))

(event `CE_Display Option`
  (if (not (`self.DisableUI`))
    (`UserWidget.AddToViewport` (`self.Option Menu`) 0)))

(event `CE_Remove Widget pause`
  (if (not (`self.DisableUI`))
    (`Widget.RemoveFromParent` (`self.Pause Menu`))))

(event `CE_Remove Option`
  (if (not (`self.DisableUI`))
    (`Widget.RemoveFromParent` (`self.Option Menu`))))

(fn `GetNewRoundMap`
  (returns (Level :type "World Soft Object Reference"))
  (bind _level (`self.Level`))
  (bind _output (`|GetArrayItem` _level))
  (`KismetArrayLibrary.Array_Shuffle` _level)
  (bind _output_get (set `self.CurrentLevel` (select `bool` (== _output (`self.CurrentLevel`)) :`false` _output :`true` (`|GetArrayItem` _level 1))))
  (return _output_get))